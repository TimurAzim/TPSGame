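; BP_Character is a top-down character that turns to face the point under the mouse cursor.
; Each tick it traces the cursor on the Visibility channel and sets only the actor's yaw toward the hit location.
; The construction script configures the camera boom's length, rotation and optional lag from Blueprint variables.
; CameraShakeIvent plays BP_CameraShake as a small-radius world shake centred on the camera.
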(event EventTick
  (params (DeltaSeconds :type Float%20%28single-precision%29))
  (Transformation|SetActorRotation (Math|Rotator|MakeRotator 0.0 0.0 (.yaw (Math|Rotator|FindLookatRotation (Transformation|GetActorLocation) (.Location (Collision|BreakHitResult (.HitResult (Game|Player|GetHitResultUnderCursorbyChannel (Game|GetPlayerController 0) "TraceTypeQuery1" true)))))))))

(fn ConstructionScript
  (bind _cameraboom (Variables|Default|GetCameraBoom))
  (Variables|/Script/Engine.SpringArmComponent|SetTargetArmLength _cameraboom (Variables|Camera|GetHieght))
  (Transformation|SetRelativeRotation _cameraboom (Variables|Camera|GetRotatorCamera) false false)
  (Variables|/Script/Engine.SpringArmComponent|SetbEnableCameraLag _cameraboom (Variables|Camera|GetFlow))
  (Variables|/Script/Engine.SpringArmComponent|SetCameraLagSpeed _cameraboom (Variables|Camera|GetCoefSmooth)))

(fn CameraShakeIvent
  (Camera|PlayWorldCameraShake "/Game/Blueprint/Game/BP_CameraShake.BP_CameraShake_C" (Transformation|GetWorldLocation (Variables|Default|GetTopDownCameraComponent)) 0.0 3e+01))